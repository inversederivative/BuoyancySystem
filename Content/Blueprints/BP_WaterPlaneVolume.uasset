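; Water volume actor that renders a water surface and applies buoyancy to physics-simulating components inside it.
; The construction script sizes the trigger box from a gizmo vector and builds the surface as a procedural grid mesh.
; Overlaps, plus a delayed BeginPlay scan, track bodies and swap their damping.
; Tick approximates submersion from each body's bounding sphere, applying upward force scaled by mass, gravity and water density.
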(event OnComponentBeginOverlap(WaterBoxTrigger)
  (params (OverlappedComponent :type Primitive%20Component%20Object%20Reference) (OtherActor :type Actor%20Object%20Reference) (OtherComp :type Primitive%20Component%20Object%20Reference) (OtherBodyIndex :type Integer) (bFromSweep :type Boolean) (SweepResult :type Hit%20Result%20Structure%20%28by%20ref%29))
  (if (Physics|IsSimulatingPhysics OtherComp "None")
    (Utilities|Array|AddUnique (Variables|Default|GetPrimitives%20List) OtherComp)
    (Class|PrimitiveComponent|SetLinearDamping OtherComp (Variables|Default|GetWater%20Linear%20Damping))
    (Class|PrimitiveComponent|SetAngularDamping OtherComp (Variables|Default|GetWater%20Angular%20Damping))))

(event OnComponentEndOverlap(WaterBoxTrigger)
  (params (OverlappedComponent :type Primitive%20Component%20Object%20Reference) (OtherActor :type Actor%20Object%20Reference) (OtherComp :type Primitive%20Component%20Object%20Reference) (OtherBodyIndex :type Integer))
  (if (Utilities|Array|ContainsItem (Variables|Default|GetPrimitives%20List) OtherComp)
    (Utilities|Array|RemoveItem (Variables|Default|GetPrimitives%20List) OtherComp)
    (Class|PrimitiveComponent|SetLinearDamping OtherComp (Variables|Default|GetNormal%20Linear%20Damping))
    (Class|PrimitiveComponent|SetAngularDamping OtherComp (Variables|Default|GetNormal%20Angular%20Damping))))

(event EventBeginPlay
  ;[1 0 0] INITIAL DETECTION HACK : If the body is already inside water volume
  (Utilities|FlowControl|Delay 0.0)
  (for _array_element (Class|PrimitiveComponent|GetOverlappingComponents (Variables|Default|GetWater%20Box%20Trigger))
    (if (Physics|IsSimulatingPhysics _array_element "None")
      (Utilities|Array|AddUnique (Variables|Default|GetPrimitives%20List) _array_element)
      (Class|PrimitiveComponent|SetLinearDamping _array_element (Variables|Default|GetWater%20Linear%20Damping))
      (Class|PrimitiveComponent|SetAngularDamping _array_element (Variables|Default|GetWater%20Angular%20Damping)))))

(event EventTick
  (params (DeltaSeconds :type Float%20%28single-precision%29))
  (Variables|Default|SetWater%20Plane%20Location (Transformation|GetActorLocation))
  (if (> (Utilities|Array|Length (Variables|Default|GetPrimitives%20List)) 0)
    (for _array_element (Variables|Default|GetPrimitives%20List)
      (Utilities|IsValid _array_element
        (:Is%20Valid
          (Class|PrimitiveComponent|AddForceatLocation _array_element (Math|Vector|MakeVector 0.0 0.0 (* (Math|Float|Clamp(Float) (/ (- (.Z (Math|Vector|BreakVector (Variables|Default|GetWater%20Plane%20Location))) (- (.Z (Math|Vector|BreakVector (.Origin (Collision|GetComponentBounds _array_element)))) (.SphereRadius (Collision|GetComponentBounds _array_element)))) (* (.SphereRadius (Collision|GetComponentBounds _array_element)) 2.0))) (Physics|GetMass _array_element) (Variables|Default|GetGravity) (Variables|Default|GetWater%20Density))) (select (> (+ (.Z (Math|Vector|BreakVector (.Origin (Collision|GetComponentBounds _array_element)))) (.SphereRadius (Collision|GetComponentBounds _array_element))) (.Z (Math|Vector|BreakVector (Variables|Default|GetWater%20Plane%20Location)))) (Math|Vector|MakeVector (.X (Math|Vector|BreakVector (.Origin (Collision|GetComponentBounds _array_element)))) (.Y (Math|Vector|BreakVector (.Origin (Collision|GetComponentBounds _array_element)))) (/ (+ (- (.Z (Math|Vector|BreakVector (.Origin (Collision|GetComponentBounds _array_element)))) (.SphereRadius (Collision|GetComponentBounds _array_element))) (.Z (Math|Vector|BreakVector (Variables|Default|GetWater%20Plane%20Location)))) 2.0)) (.Origin (Collision|GetComponentBounds _array_element))) "None"))))))

(fn ConstructionScript
  (bind _num_vertices_y (Variables|Default|GetNum%20Vertices%20Y))
  (bind _num_vertices_x (Variables|Default|GetNum%20Vertices%20X))
  (bind _returnvalue (- _num_vertices_y 1))
  (bind _returnvalue_2 (- _num_vertices_x 1))
  (Utilities|FlowControl|Sequence
    (:then_0
      ;[1 1 1] c1_1
      (Variables|Default|SetWater%20Volume%20Gizmo (Math|Vector|MakeVector (Math|Float|Max(Float) (.X (Math|Vector|BreakVector (Variables|Default|GetWater%20Volume%20Gizmo))) 1e+02) (Math|Float|Max(Float) (.Y (Math|Vector|BreakVector (Variables|Default|GetWater%20Volume%20Gizmo))) 1e+02) (Math|Float|Min(Float) (.Z (Math|Vector|BreakVector (Variables|Default|GetWater%20Volume%20Gizmo))) -1e+02)))
      (Components|Box|SetBoxExtent (Variables|Default|GetWater%20Box%20Trigger) (Math|Vector|MakeVector (Math|Float|Absolute(Float) (.X (Math|Vector|BreakVector (/ (Variables|Default|GetWater%20Volume%20Gizmo) 2.0)))) (Math|Float|Absolute(Float) (.Y (Math|Vector|BreakVector (/ (Variables|Default|GetWater%20Volume%20Gizmo) 2.0)))) (Math|Float|Absolute(Float) (.Z (Math|Vector|BreakVector (/ (Variables|Default|GetWater%20Volume%20Gizmo) 2.0))))) true)
      (Transformation|SetRelativeLocation (Variables|Default|GetWater%20Box%20Trigger) (/ (Variables|Default|GetWater%20Volume%20Gizmo) 2.0) false false))
    (:then_1
      (Utilities|Array|Clear (Variables|Default|GetVertices))
      (Utilities|Array|Clear (Variables|Default|GetTriangles))
      (Utilities|Array|Clear (Variables|Default|GetUV0))
      (Utilities|Array|Clear (Variables|Default|GetNormals))
      (Utilities|Array|Clear (Variables|Default|GetVertex%20Colors))
      (Utilities|Array|Clear (Variables|Default|GetTangents)))
    (:then_2
      ;[1 1 1] 3_1
      (for _index (range 0 _returnvalue_2)
        (LocalVariables|SetX _index)
        ;[1 1 1] 3_2
        (for _index_2 (range 0 _returnvalue)
          (LocalVariables|SetY _index_2)
          (Utilities|Array|Add (Variables|Default|GetVertices) (Math|Vector|MakeVector (* (/ (Math|Conversions|ToFloat(Integer) (LocalVariables|GetX)) (Math|Conversions|ToFloat(Integer) _returnvalue_2)) (.X (Math|Vector|BreakVector (Variables|Default|GetWater%20Volume%20Gizmo)))) (* (.Y (Math|Vector|BreakVector (Variables|Default|GetWater%20Volume%20Gizmo))) (/ (Math|Conversions|ToFloat(Integer) (LocalVariables|GetY)) (Math|Conversions|ToFloat(Integer) _returnvalue))) (* (Variables|Default|GetMesh%20vertical%20Offset) -1.0)))
          (Utilities|Array|Add (Variables|Default|GetUV0) (Math|Vector2D|MakeVector2D (/ (Math|Conversions|ToFloat(Integer) (LocalVariables|GetX)) (Math|Conversions|ToFloat(Integer) _returnvalue_2)) (/ (Math|Conversions|ToFloat(Integer) (LocalVariables|GetY)) (Math|Conversions|ToFloat(Integer) _returnvalue))))
          (Utilities|Array|Add (Variables|Default|GetVertex%20Colors) (Variables|Default|GetVertex%20Color)))))
    (:then_3
      (bind _triangles (Class|KismetProceduralMeshLibrary|CreateGridMeshTriangles (Variables|Default|GetNum%20Vertices%20X) (Variables|Default|GetNum%20Vertices%20Y) false))
      (Variables|Default|SetTriangles _triangles)
      (bind (_normals _tangents) (Class|KismetProceduralMeshLibrary|CalculateTangentsforMesh (Variables|Default|GetVertices) (Variables|Default|GetTriangles) (Variables|Default|GetUV0)))
      (Variables|Default|SetNormals _normals)
      (Variables|Default|SetTangents _tangents))
    (:then_4
      (Class|ProceduralMeshComponent|CreateMeshSectionLinearColor (Variables|Default|GetWaterProceduralMesh) 0 (Variables|Default|GetVertices) (Variables|Default|GetTriangles) (Variables|Default|GetNormals) (Variables|Default|GetUV0) 0 0 0 (Variables|Default|GetVertex%20Colors) (Variables|Default|GetTangents) false)
      (Rendering|Material|SetMaterial (Variables|Default|GetWaterProceduralMesh) 0 (Variables|Default|GetWater%20Material)))))