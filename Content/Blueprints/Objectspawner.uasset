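; Object spawner that continuously emits physics-simulated props of random shape and size at its own location.
; On BeginPlay it starts an endless loop that adds a static mesh component, picks a random mesh from the Staticmesh array, enables physics and applies a random uniform scale.
; A short random delay separates iterations, and the spawned components accumulate on the same Blueprint, with no limit or cleanup.
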(event EventBeginPlay
  (bind _staticmesh (Variables|Default|Getstaticmesh))
  (bind _returnvalue (AddComponent|AddStaticMeshComponent false (Math|Transform|MakeTransform "0, 0, 0") :!label _label))
  (Components|StaticMesh|SetStaticMesh _returnvalue (Utilities|Array|Get(acopy) _staticmesh (Math|Random|RandomIntegerinRange 0 (Utilities|Array|LastIndex _staticmesh))))
  (Physics|SetSimulatePhysics _returnvalue true)
  (Transformation|SetRelativeScale3D _returnvalue (Math|Conversions|ToVector(Float) (Math|Random|RandomFloatinRange 0.1 4.0)))
  (Utilities|FlowControl|Delay (Math|Random|RandomFloatinRange 0.5 1.0))
  (goto _label))

(fn ConstructionScript)